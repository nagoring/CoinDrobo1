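; BP_EnemyCharacter is an enemy that chases the player and drains HP on contact.
; From BeginPlay it loops, reissuing AIMoveTo toward player pawn 0 after a short delay.
; Any capsule hit, without checking what was struck, decrements HP stored in BP_GameInstance.
; When that HP runs out, it opens level Hello5_3.
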(event OnComponentHit(CapsuleComponent)
  (params (HitComponent :type Primitive%20Component%20Object%20Reference) (OtherActor :type Actor%20Object%20Reference) (OtherComp :type Primitive%20Component%20Object%20Reference) (NormalImpulse :type Vector :default "0, 0, 0") (Hit :type Hit%20Result%20Structure%20%28by%20ref%29))
  (bind _returnvalue (Game|GetGameInstance))
  (bind _asbp_game_instance (Utilities|Casting|CastToBP_GameInstance _returnvalue))
  (bind _output_get (Variables|/Game/BP/BP_GameInstance.BP_GameInstance_C|SetHP _asbp_game_instance (- (Variables|/Game/BP/BP_GameInstance.BP_GameInstance_C|GetHP _asbp_game_instance) 1)))
  (if (<= _output_get 0)
    (Game|OpenLevel(byName) "Hello5_3")))

(event EventBeginPlay
  (AI|AIMoveTo self "0, 0, 0" (Game|Player|GetPlayerPawn 0) 5.0 false :!label _label
    (:then
      (Utilities|FlowControl|Delay 0.2)
      (goto _label))))

(event Collision|EventActorBeginOverlap
  (params (OtherActor :type Actor%20Object%20Reference)))

(event EventTick
  (params (DeltaSeconds :type Float%20%28single-precision%29)))

(fn ConstructionScript)